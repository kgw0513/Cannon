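; BP_Cannon is a player-operable cannon that fires BP_CannonBall projectiles.
; Entering its box enables input and shows an E prompt; E toggles control, blending the camera to the cannon and disabling player input.
; While controlled, axis inputs rotate the Middle component within angle limits, and Space hold time sets clamped launch speed on release.
; Leaving the box restores the player; the three-second fire cooldown is unconnected.
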(event OnComponentBeginOverlap(Box)
  (params (OverlappedComponent :type Primitive%20Component%20Object%20Reference) (OtherActor :type Actor%20Object%20Reference) (OtherComp :type Primitive%20Component%20Object%20Reference) (OtherBodyIndex :type Integer) (bFromSweep :type Boolean) (SweepResult :type Hit%20Result%20Structure%20%28by%20ref%29))
  (if (Class|GameplayStatics|ObjectIsA OtherActor "/Game/ThirdPerson/Blueprints/BP_ThirdPersonCharacter.BP_ThirdPersonCharacter_C")
    (bind _asbp_third_person_character (Utilities|Casting|CastToBP_ThirdPersonCharacter OtherActor))
    (Variables|Default|SetPlayer _asbp_third_person_character)
    (Input|EnableInput (Game|GetPlayerController 0))
    (UserInterface|SetWidget (Variables|Default|GetPressWidget) (Variables|Default|GetKeyShowE))))

(event OnComponentEndOverlap(Box)
  (params (OverlappedComponent :type Primitive%20Component%20Object%20Reference) (OtherActor :type Actor%20Object%20Reference) (OtherComp :type Primitive%20Component%20Object%20Reference) (OtherBodyIndex :type Integer))
  (bind _returnvalue (Game|GetPlayerController 0))
  (if (== OtherActor (Variables|Default|GetPlayer))
    (Input|EnableInput (Variables|Default|GetPlayer) 0)
    (Game|Player|SetViewTargetwithBlend (Game|GetPlayerController 0) (Variables|Default|GetPlayer) 1.0 "VTBlend_Linear" 0.0 false)
    (Input|EnableInput (Variables|Default|GetPlayer) _returnvalue)
    (Variables|Default|SetbNowControl false)
    (Variables|Default|SetbNowFire false)
    (Variables|Default|SetPlayer 0)
    (Input|DisableInput _returnvalue)
    (UserInterface|SetWidget (Variables|Default|GetPressWidget) 0)))

(event EventBeginPlay
  (bind _returnvalue (UserInterface|CreateWidget "/Game/Cannon/WBP_KeyE.WBP_KeyE_C"))
  (Variables|Default|SetKeyShowE _returnvalue))

(event Input|AxisEvents|InputAxisMoveCannonLR
  (params (AxisValue :type Float%20%28single-precision%29))
  (bind _middle (Variables|Default|GetMiddle))
  (bind _relativerotation (Variables|/Script/Engine.SceneComponent|GetRelativeRotation _middle))
  (if (Variables|Default|GetbNowControl)
    (Transformation|SetRelativeRotation (Variables|Default|GetMiddle) (Math|Rotator|MakeRotator 0.0 (.pitch _relativerotation) (Math|Float|ClampAngle (+ (.yaw _relativerotation) AxisValue) (Variables|Default|GetMinAngleLR) (Variables|Default|GetMaxAngleLR))) false false)))

(event Input|AxisEvents|InputAxisMoveCannonUD
  (params (AxisValue :type Float%20%28single-precision%29))
  (bind _middle (Variables|Default|GetMiddle))
  (bind _relativerotation (Variables|/Script/Engine.SceneComponent|GetRelativeRotation _middle))
  (if (Variables|Default|GetbNowControl)
    (Transformation|SetRelativeRotation (Variables|Default|GetMiddle) (Math|Rotator|MakeRotator 0.0 (Math|Float|ClampAngle (+ (.pitch _relativerotation) AxisValue) (Variables|Default|GetMinAngleUD) (Variables|Default|GetMaxAngleUD)) (.yaw _relativerotation)) false false)))

(event Input|KeyboardEvents|E
  (params (Key :type Key%20Structure :default "None"))
  (bind _returnvalue (Game|GetPlayerController 0))
  (:Pressed
    (Utilities|FlowControl|FlipFlop
      (:A
        (Game|Player|SetViewTargetwithBlend _returnvalue self 0.4 "VTBlend_Linear" 0.0 true)
        (Variables|Default|SetbNowControl true)
        (Input|DisableInput (Variables|Default|GetPlayer) (Game|GetPlayerController 0))
        (UserInterface|SetWidget (Variables|Default|GetPressWidget) 0))
      (:B
        (Game|Player|SetViewTargetwithBlend _returnvalue (Variables|Default|GetPlayer) 0.4 "VTBlend_Linear" 0.0 true)
        (Variables|Default|SetbNowControl false)
        (Input|EnableInput (Variables|Default|GetPlayer) (Game|GetPlayerController 0))
        (UserInterface|SetWidget (Variables|Default|GetPressWidget) (Variables|Default|GetKeyShowE))))))

(event Input|KeyboardEvents|SpaceBar
  (params (Key :type Key%20Structure :default "None"))
  (bind _returnvalue (Actor|GetGameTimeSinceCreation))
  (:Pressed
    (Variables|Default|SetPressedTime _returnvalue))
  (:Released
    (Variables|Default|SetRePressedTime _returnvalue)
    (if (and (Variables|Default|GetbNowControl) (not (Variables|Default|GetbNowFire)))
      (Variables|Default|SetMaxTime (Math|Float|Clamp(Float) (* (- (Variables|Default|GetRePressedTime) (Variables|Default|GetPressedTime)) 1e+03) 5e+02 2e+03))
      (bind _returnvalue_2 (Game|SpawnActorfromClass "/Game/Cannon/BP_CannonBall.BP_CannonBall_C" (Transformation|GetWorldTransform (Variables|Default|GetStaticMesh)) "AlwaysSpawn" "MultiplyWithRoot" 0 0))
      (Variables|/Script/Engine.ProjectileMovementComponent|SetInitialSpeed (Variables|/Game/Cannon/BP_CannonBall.BP_CannonBall_C|GetCannonBallPhysic _returnvalue_2) (Variables|Default|GetMaxTime))
      (Variables|/Script/Engine.ProjectileMovementComponent|SetMaxSpeed (Variables|/Game/Cannon/BP_CannonBall.BP_CannonBall_C|GetCannonBallPhysic _returnvalue_2) (Variables|Default|GetMaxTime)))))

(fn ConstructionScript)